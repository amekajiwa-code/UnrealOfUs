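; Maze generator actor that, on BeginPlay, builds a random square grid maze of BP_Cell actors and populates it with items and enemies.
; Cells keep west and north walls only on the outer border.
; A binary tree pass randomly opens each cell's east or south wall, switching direction at the far edges.
; Items and Enemy_Character monsters then spawn at random cells, CellCount of each, with Enemy_Controller set as the monsters' AI controller class.
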(event EventBeginPlay
  (bind _interval (Variables|Default|Getinterval))
  (bind _cellcount (Variables|Default|GetCellCount))
  (bind _interval_2 (Variables|Default|Getinterval))
  (bind _returnvalue (* _cellcount _interval_2))
  (bind _returnvalue_2 (- _returnvalue _interval_2))
  ;[1 1 1] Generate Map
  (for _index (range 1 (Variables|Default|GetCellCount))
    (for _index_2 (range 1 (Variables|Default|GetCellCount))
      (bind _returnvalue_3 (Game|SpawnActorfromClass "/Game/BP/Maze/BP_Cell.BP_Cell_C" (Math|Conversions|ToTransform(Vector) (Variables|Default|GetNextPos)) "Undefined" "MultiplyWithRoot" 0 0))
      (Variables|Default|SetNextPos (+ (Variables|Default|GetNextPos) (Math|Vector|MakeVector (Variables|Default|Getinterval) 0.0 0.0)))
      (Utilities|Array|Insert (Variables|Default|GetCellList) _returnvalue_3))
    (Variables|Default|SetNextPos (+ (Variables|Default|GetNextPos) (Math|Vector|MakeVector (* (Variables|Default|GetCellCount) (* _interval -1.0)) _interval 0.0))))
  ;[1 1 1] Binary Tree Map
  (for _array_element (Variables|Default|GetCellList)
    (Utilities|FlowControl|Sequence
      (:then_0
        (if (== (.x (Math|Transform|TransformLocation (Transformation|GetActorTransform _array_element) "0, 0, 0")) 0.0)
          (Default|SetWWall _array_element true)
          (else
            (Default|SetWWall _array_element false))))
      (:then_1
        (if (== (.y (Math|Transform|TransformLocation (Transformation|GetActorTransform _array_element) "0, 0, 0")) 0.0)
          (Default|SetNWall _array_element true)
          (else
            (Default|SetNWall _array_element false))))
      (:then_2
        (switch int (Math|Random|RandomIntegerinRange 0 1)
          (:0
            (if (<= (+ (.x (Math|Transform|TransformLocation (Transformation|GetActorTransform _array_element) "0, 0, 0")) _interval_2) _returnvalue_2)
              (Default|SetEWall _array_element false)
              (else
                (Default|SetSWall _array_element false))))
          (:1
            (if (<= (+ (.y (Math|Transform|TransformLocation (Transformation|GetActorTransform _array_element) "0, 0, 0")) _interval_2) _returnvalue_2)
              (Default|SetSWall _array_element false)
              (else
                (Default|SetEWall _array_element false))))))))
  ;[1 1 1] Item Spawn
  (for _index_3 (range 1 (Variables|Default|GetCellCount))
    (Game|SpawnActorfromClass "/Game/BP/BP_Item.BP_Item_C" (Math|Conversions|ToTransform(Vector) (Math|Transform|TransformLocation (Transformation|GetActorTransform (.OutItem (Utilities|Array|Random (Variables|Default|GetCellList)))) "0, 0, 0")) "Undefined" "MultiplyWithRoot" 0 0))
  ;[1 1 1] Spawn Monster
  (for _index_4 (range 1 (Variables|Default|GetCellCount))
    (bind _returnvalue_4 (Game|SpawnActorfromClass "/Game/BP/Enemy/Enemy_Character.Enemy_Character_C" (Math|Conversions|ToTransform(Vector) (Math|Transform|TransformLocation (Transformation|GetActorTransform (.OutItem (Utilities|Array|Random (Variables|Default|GetCellList)))) "0, 0, 0")) "Undefined" "MultiplyWithRoot" 0 0))
    (Variables|/Script/Engine.Pawn|SetAIControllerClass _returnvalue_4 "/Game/BP/Enemy/Enemy_Controller.Enemy_Controller_C")))

(fn ConstructionScript)