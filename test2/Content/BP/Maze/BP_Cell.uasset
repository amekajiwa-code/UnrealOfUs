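; BP_Cell is a maze cell with four walls (N, S, E, W), each toggled by its own setter event.
; Each setter stores a visibility flag and applies it to the wall's visibility and collision, so hidden walls are passable.
; BeginPlay repeatedly picks a random wall and passes that wall's current flag to its setter, without inverting it.
; IsVisited infers visited state from the flags, returning true once any wall is hidden.
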(event Custom|Set%20W_Wall
  (params (Visibility :type Boolean))
  (bind _w_wall (Variables|Default|GetW_Wall))
  ;[1 1 1] SET Wall Event
  (bind _output_get (Variables|Default|SetisVisivleW Visibility))
  (Rendering|SetVisibility _w_wall _output_get true)
  (Collision|SetCollisionEnabled _w_wall (select _output_get "QueryAndPhysics" "NoCollision")))

(event Custom|Set%20N_Wall
  (params (Visibility :type Boolean))
  (bind _n_wall (Variables|Default|GetN_Wall))
  ;[1 1 1] SET Wall Event
  (bind _output_get (Variables|Default|SetisVisivleN Visibility))
  (Rendering|SetVisibility _n_wall _output_get true)
  (Collision|SetCollisionEnabled _n_wall (select _output_get "QueryAndPhysics" "NoCollision")))

(event Custom|Set%20S_Wall
  (params (Visibility :type Boolean))
  (bind _s_wall (Variables|Default|GetS_Wall))
  ;[1 1 1] SET Wall Event
  (bind _output_get (Variables|Default|SetisVisivleS Visibility))
  (Rendering|SetVisibility _s_wall _output_get true)
  (Collision|SetCollisionEnabled _s_wall (select _output_get "QueryAndPhysics" "NoCollision")))

(event Custom|Set%20E_Wall
  (params (Visibility :type Boolean))
  (bind _e_wall (Variables|Default|GetE_Wall))
  ;[1 1 1] SET Wall Event
  (bind _output_get (Variables|Default|SetisVisivleE Visibility))
  (Rendering|SetVisibility _e_wall _output_get true)
  (Collision|SetCollisionEnabled _e_wall (select _output_get "QueryAndPhysics" "NoCollision")))

(event EventBeginPlay
  (for _index (range 0 2)
    (switch int (Math|Random|RandomIntegerinRange 0 3)
      (:0
        (CallFunction|SetNWall (Variables|Default|GetisVisivleN)))
      (:1
        (CallFunction|SetSWall (Variables|Default|GetisVisivleS)))
      (:2
        (CallFunction|SetEWall (Variables|Default|GetisVisivleE)))
      (:3
        (CallFunction|SetWWall (Variables|Default|GetisVisivleW))))))

(fn ConstructionScript)

(fn IsVisited
  (return (not (Math|Boolean|ANDBoolean (Variables|Default|GetisVisivleN) (Variables|Default|GetisVisivleS) (Variables|Default|GetisVisivleE) (Variables|Default|GetisVisivleW)))))