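; BP_Item is a collectible actor that tracks how many items remain through an ItemCount on MyGameMode.
; On BeginPlay it registers itself by incrementing the count.
; The first overlap by any actor hides it and decrements the count, with the HiddenMode flag preventing repeat triggers.
; The item is only hidden, never destroyed.
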(event Collision|EventActorBeginOverlap
  (params (OtherActor :type Actor%20Object%20Reference))
  (if (not (Variables|Default|GetHiddenMode))
    (bind _output_get (Variables|Default|SetHiddenMode (not (Variables|Default|GetHiddenMode))))
    (Rendering|SetActorHiddenInGame _output_get)
    (bind _asmy_game_mode (Utilities|Casting|CastToMyGameMode (Game|GetGameMode)))
    (Variables|/Game/BP/MyGameMode.MyGameMode_C|SetItemCount _asmy_game_mode (- (Variables|/Game/BP/MyGameMode.MyGameMode_C|GetItemCount _asmy_game_mode) 1))))

(event EventBeginPlay
  (bind _asmy_game_mode (Utilities|Casting|CastToMyGameMode (Game|GetGameMode)))
  (Variables|/Game/BP/MyGameMode.MyGameMode_C|SetItemCount _asmy_game_mode (+ (Variables|/Game/BP/MyGameMode.MyGameMode_C|GetItemCount _asmy_game_mode) 1)))

(fn ConstructionScript)